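; BP_JumpLand is an animation notify that plays a landing sound matched to the surface under the shooter character.
; When triggered, it casts the mesh owner to BP_ShooterCharacter and queries that character's surface type.
; A switch selects the metal, stone, tile, grass or water sound, defaulting to tile, and plays it at the owner's location.
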(fn ReceivedNotify
  (params (MeshComp :type Skeletal%20Mesh%20Component%20Object%20Reference) (Animation :type Anim%20Sequence%20Base%20Object%20Reference) (EventReference :type Anim%20Notify%20Event%20Reference%20Structure%20%28by%20ref%29))
  (bind _returnvalue (Components|GetOwner MeshComp))
  (bind _asbp_shooter_character (Utilities|Casting|CastToBP_ShooterCharacter _returnvalue))
  (bind _returnvalue_2 (Class|ShooterCharacter|GetSurfaceType _asbp_shooter_character))
  (switch Utilities|FlowControl|Switch|SwitchonEPhysicalSurface _returnvalue_2
    (:SurfaceType_Default
      (LocalVariables|SetLanding%20Sound "/Game/_Game/Assets/Audio/MetaSounds/Jump/sfx_JumpLandTile.sfx_JumpLandTile"))
    (:SurfaceType1
      (LocalVariables|SetLanding%20Sound "/Game/_Game/Assets/Audio/MetaSounds/Jump/sfx_JumpLandMetal.sfx_JumpLandMetal"))
    (:SurfaceType2
      (LocalVariables|SetLanding%20Sound "/Game/_Game/Assets/Audio/MetaSounds/Jump/sfx_JumpLandStone.sfx_JumpLandStone"))
    (:SurfaceType3
      (LocalVariables|SetLanding%20Sound "/Game/_Game/Assets/Audio/MetaSounds/Jump/sfx_JumpLandTile.sfx_JumpLandTile"))
    (:SurfaceType4
      (LocalVariables|SetLanding%20Sound "/Game/_Game/Assets/Audio/MetaSounds/Jump/sfx_JumpLandGrass.sfx_JumpLandGrass"))
    (:SurfaceType5
      (LocalVariables|SetLanding%20Sound "/Game/_Game/Assets/Audio/MetaSounds/Jump/sfx_JumpLandWater.sfx_JumpLandWater")))
  (Audio|PlaySoundatLocation (LocalVariables|GetLanding%20Sound) (Transformation|GetActorLocation _returnvalue) "0, 0, 0" 1.0 1.0 0.0 0 0 0 0)
  (return false))
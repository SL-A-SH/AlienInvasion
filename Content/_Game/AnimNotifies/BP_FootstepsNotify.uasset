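; Footstep anim notify that plays surface-specific sound and Niagara effects for BP_ShooterCharacter during animations.
; It asks the owning character for its surface type and picks a matching sound and particle system, falling back to metal for unhandled surfaces.
; Both spawn at the location of the socket named by BoneName on the animated mesh.
; Meshes owned by other actor types are ignored.
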(fn ReceivedNotify
  (params (MeshComp :type Skeletal%20Mesh%20Component%20Object%20Reference) (Animation :type Anim%20Sequence%20Base%20Object%20Reference) (EventReference :type Anim%20Notify%20Event%20Reference%20Structure%20%28by%20ref%29))
  (bind _bonename (Variables|Default|GetBoneName))
  (bind _returnvalue (Transformation|GetSocketLocation MeshComp _bonename))
  (bind _asbp_shooter_character (Utilities|Casting|CastToBP_ShooterCharacter (Components|GetOwner MeshComp)))
  (bind _returnvalue_2 (Class|ShooterCharacter|GetSurfaceType _asbp_shooter_character))
  (switch Utilities|FlowControl|Switch|SwitchonEPhysicalSurface _returnvalue_2
    (:SurfaceType_Default
      (LocalVariables|SetFootstepSound "/Game/_Game/Assets/Audio/MetaSounds/sfx_FootstepMetal.sfx_FootstepMetal")
      (LocalVariables|SetFootstepNiagaraSystem "/Game/A_Surface_Footstep/Niagara_FX/ParticleSystems/PSN_General1_Surface.PSN_General1_Surface"))
    (:SurfaceType1
      (LocalVariables|SetFootstepSound "/Game/_Game/Assets/Audio/MetaSounds/sfx_FootstepMetal.sfx_FootstepMetal")
      (LocalVariables|SetFootstepNiagaraSystem "/Game/A_Surface_Footstep/Niagara_FX/ParticleSystems/PSN_General1_Surface.PSN_General1_Surface"))
    (:SurfaceType2
      (LocalVariables|SetFootstepSound "/Game/_Game/Assets/Audio/MetaSounds/sfx_FootstepStone.sfx_FootstepStone")
      (LocalVariables|SetFootstepNiagaraSystem "/Game/A_Surface_Footstep/Niagara_FX/ParticleSystems/PSN_Gravel_Surface.PSN_Gravel_Surface"))
    (:SurfaceType3
      (LocalVariables|SetFootstepSound "/Game/_Game/Assets/Audio/MetaSounds/sfx_FootstepTile.sfx_FootstepTile")
      (LocalVariables|SetFootstepNiagaraSystem "/Game/A_Surface_Footstep/Niagara_FX/ParticleSystems/PSN_General2_Surface.PSN_General2_Surface"))
    (:SurfaceType4
      (LocalVariables|SetFootstepSound "/Game/_Game/Assets/Audio/MetaSounds/sfx_FootstepGrass.sfx_FootstepGrass")
      (LocalVariables|SetFootstepNiagaraSystem "/Game/A_Surface_Footstep/Niagara_FX/ParticleSystems/PSN_Grass_Surface.PSN_Grass_Surface"))
    (:SurfaceType5
      (LocalVariables|SetFootstepSound "/Game/_Game/Assets/Audio/MetaSounds/sfx_FootstepWater.sfx_FootstepWater")
      (LocalVariables|SetFootstepNiagaraSystem "/Game/A_Surface_Footstep/Niagara_FX/ParticleSystems/PSN_WaterLight_Surface.PSN_WaterLight_Surface")))
  (Audio|PlaySoundatLocation (LocalVariables|GetFootstepSound) _returnvalue "0, 0, 0" 1.0 1.0 0.0 0 0 0 0)
  (Niagara|SpawnSystematLocation (LocalVariables|GetFootstepNiagaraSystem) _returnvalue)
  (return false))